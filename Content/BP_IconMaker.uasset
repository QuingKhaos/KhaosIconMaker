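; BP_IconMaker is an editor tool that renders and saves icon textures for buildables, items or static meshes.
; Construction or ForceUpdate feeds the first valid subject to a capture actor, applies camera and light settings, and derives a UI/IconDesc_ export name from the asset path.
; Export draws an M_InvertAlpha dynamic material into each render target and saves the result as a resolution-suffixed texture asset.
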(fn `Export`
  (if (`KismetStringLibrary.IsEmpty` (`self.mExportName`))
    (return)
    (else
      (for _array_element (`self.mExportTargets`)
        (`self.ExportRender` _array_element (`KismetStringLibrary.Conv_IntToString` (`TextureRenderTarget2D.SizeX` _array_element))))
      (return))))

(fn `ExportRender`
  (params (ExportTarget :type "TextureRenderTarget2D Object Reference") (Resolution :type String))
  (locals (OriginalExportCapture :type "TextureRenderTarget2D Object Reference"))
  (bind _returnvalue (`KismetStringLibrary.Concat_StrStr` (`self.mExportName`) "_" Resolution))
  (`KismetRenderingLibrary.ClearRenderTarget2D` null ExportTarget (struct))
  (`KismetRenderingLibrary.DrawMaterialToRenderTarget` null ExportTarget (`self.ExportMaterial`))
  (bind _returnvalue_2 (`KismetRenderingLibrary.RenderTargetCreateStaticTexture2DEditorOnly` ExportTarget _returnvalue))
  (set `Texture.SRGB` true _returnvalue_2)
  (set `Texture.LODGroup` "TEXTUREGROUP_Project01" _returnvalue_2)
  (bind _returnvalue_3 (`GeometryScriptLibrary_CreateNewAssetFunctions.CreateNewTexture2DAsset` _returnvalue_2 _returnvalue (make `GeometryScriptCreateNewTexture2DAssetOptions` true) null)
    (:`Failure`
      _)
    (:`Success`
      (`EditorAssetLibrary.SaveLoadedAsset` _returnvalue_3 false)))
  (return))

(fn `ForceUpdate`
  (`self.UpdateAll`)
  (bind _returnvalue (`KismetMaterialLibrary.CreateDynamicMaterialInstance` null "/KhaosIconMaker/Capture/M_InvertAlpha.M_InvertAlpha"))
  (set `self.ExportMaterial` _returnvalue)
  (return))

(fn `GetBuildableName`
  (params (Buildable :type "FGBuildable Class Reference"))
  (returns (FullName :type String))
  (locals (ClassDisplayName :type String) (ItemName :type String) (ClassPath :type String))
  (bind _classdisplayname (`local.ClassDisplayName`))
  (`|ExecutionSequence`
    (:`then_0`
      (bind _output_get (set `local.ClassDisplayName` (`KismetSystemLibrary.GetClassDisplayName` Buildable)))
      (set `local.ItemName` (`KismetStringLibrary.Replace` (`KismetStringLibrary.Replace` _output_get "Build_") "_C")))
    (:`then_1`
      (set `local.ClassPath` (`KismetStringLibrary.Replace` (`KismetStringLibrary.Replace` (`KismetStringLibrary.Replace` (`KismetSystemLibrary.BreakTopLevelAssetPath` (`KismetSystemLibrary.GetClassTopLevelAssetPath` Buildable)) _classdisplayname) (`KismetStringLibrary.GetSubstring` _classdisplayname 0 (- (`KismetStringLibrary.Len` _classdisplayname) 2))) ".")))
    (:`then_2`
      (return (`KismetStringLibrary.Concat_StrStr` (`local.ClassPath`) "UI/IconDesc_" (`local.ItemName`))))))

(fn `GetItemName`
  (params (ItemDesc :type "FGItemDescriptor Class Reference"))
  (returns (FullName :type String))
  (locals (ClassDisplayName :type String) (ClassPath :type String) (ItemName :type String))
  (bind _classdisplayname (`local.ClassDisplayName`))
  (`|ExecutionSequence`
    (:`then_0`
      (bind _output_get (set `local.ClassDisplayName` (`KismetSystemLibrary.GetClassDisplayName` ItemDesc)))
      (set `local.ItemName` (`KismetStringLibrary.Replace` (`KismetStringLibrary.Replace` _output_get "Desc_") "_C")))
    (:`then_1`
      (set `local.ClassPath` (`KismetStringLibrary.Replace` (`KismetStringLibrary.Replace` (`KismetStringLibrary.Replace` (`KismetSystemLibrary.BreakTopLevelAssetPath` (`KismetSystemLibrary.GetClassTopLevelAssetPath` ItemDesc)) _classdisplayname) (`KismetStringLibrary.GetSubstring` _classdisplayname 0 (- (`KismetStringLibrary.Len` _classdisplayname) 2))) ".")))
    (:`then_2`
      (return (`KismetStringLibrary.Concat_StrStr` (`local.ClassPath`) "UI/IconDesc_" (`local.ItemName`))))))

(fn `GetMeshName`
  (params (StaticMesh :type "StaticMesh Object Reference"))
  (returns (FullName :type String))
  (locals (ObjectName :type String) (ObjectPath :type String) (ItemName :type String))
  (bind _returnvalue (`KismetSystemLibrary.GetPathName` StaticMesh))
  (bind _returnvalue_2 (`KismetSystemLibrary.GetPathName` StaticMesh))
  (bind _returnvalue_3 (`KismetStringLibrary.FindSubstring` _returnvalue_2 "SM_" true true))
  (`|ExecutionSequence`
    (:`then_0`
      (bind _output_get (set `local.ObjectName` (`KismetStringLibrary.GetSubstring` _returnvalue_2 _returnvalue_3 (- (`KismetStringLibrary.Len` _returnvalue_2) _returnvalue_3))))
      (set `local.ItemName` (`KismetStringLibrary.Replace` _output_get "SM_")))
    (:`then_1`
      (set `local.ObjectPath` (`KismetStringLibrary.GetSubstring` _returnvalue 0 (`KismetStringLibrary.FindSubstring` (`KismetStringLibrary.Replace` _returnvalue "Meshes/") "SM_" true))))
    (:`then_2`
      (return (`KismetStringLibrary.Concat_StrStr` (`local.ObjectPath`) "UI/IconDesc_" (`local.ItemName`))))))

(fn `ResetAll`
  (set `self.mBuildingClass` null)
  (set `self.mItemClass` null)
  (set `self.mItemMesh` null)
  (`/KhaosIconMaker/Capture/BP_Capture.ClearCapture` (`self.mCaptureActor`)))

(fn `UpdateAll`
  (`self.UpdateCapture`)
  (`self.UpdateCamera`)
  (`self.UpdateLight`)
  (`self.UpdateName`)
  (return))

(fn `UpdateCamera`
  (set `SpringArmComponent.TargetArmLength` (`self.mCameraArm`) (`self.mArm`))
  (`SceneComponent.K2_SetRelativeRotation` (`self.mArm`) (`self.mCameraRotation`) false false)
  (bind _output_get (set `SceneCaptureComponent2D.FOVAngle` (`self.mFOVAngle`) (`self.mExportCapture`)))
  (`CameraComponent.SetFieldOfView` (`self.mWindowPreview`) _output_get)
  (`SceneComponent.K2_SetRelativeLocation` (`self.mArm`) (`self.mCameraLocation`) false false)
  (`CameraComponent.SetAspectRatio` (`self.mWindowPreview`) 1.0))

(fn `UpdateCapture`
  (if (`KismetSystemLibrary.IsValidClass` (`self.mBuildingClass`))
    (`/KhaosIconMaker/Capture/BP_Capture.SetBuildableCapture` (`self.mCaptureActor`) (`self.mBuildingClass`) (`self.mPrimaryColor`) (`self.mSecondaryColor`) (`self.mProductionIndicatorState`))
    (return)
    (elif (`KismetSystemLibrary.IsValidClass` (`self.mItemClass`))
      (`/KhaosIconMaker/Capture/BP_Capture.SetItemCapture` (`self.mCaptureActor`) (`self.mItemClass`))
      (return)
      (elif (`KismetSystemLibrary.IsValid` (`self.mItemMesh`))
        (`/KhaosIconMaker/Capture/BP_Capture.SetMeshCapture` (`self.mCaptureActor`) (`self.mItemMesh`))
        (return)
        (else
          (`/KhaosIconMaker/Capture/BP_Capture.ClearCapture` (`self.mCaptureActor`))
          (return))))))

(fn `UpdateLight`
  (`LightComponent.SetIntensity` (`Light.LightComponent` (`self.mLight`)) (`self.mLightIntensity`))
  (`SceneComponent.K2_SetWorldRotation` (`Light.LightComponent` (`self.mLight`)) (`KismetMathLibrary.SelectRotator` (`KismetMathLibrary.FindLookAtRotation` (`SceneComponent.K2_GetComponentLocation` (`self.mWindowPreview`)) (`SceneComponent.K2_GetComponentLocation` (`self.mArm`))) (`self.mLightRotation`) (`self.mUseCameraToActorRotation`)) false false))

(fn `UpdateName`
  (if (`KismetSystemLibrary.IsValidClass` (`self.mBuildingClass`))
    (bind _fullname (`self.GetBuildableName` (`self.mBuildingClass`)))
    (set `self.mExportName` _fullname)
    (return)
    (elif (`KismetSystemLibrary.IsValidClass` (`self.mItemClass`))
      (bind _fullname_2 (`self.GetItemName` (`self.mItemClass`)))
      (set `self.mExportName` _fullname_2)
      (return)
      (elif (`KismetSystemLibrary.IsValid` (`self.mItemMesh`))
        (bind _fullname_3 (`self.GetMeshName` (`self.mItemMesh`)))
        (set `self.mExportName` _fullname_3)
        (return)
        (else
          (set `self.mExportName` "")
          (return))))))

(fn `UserConstructionScript`
  (`self.UpdateAll`)
  (bind _returnvalue (`KismetMaterialLibrary.CreateDynamicMaterialInstance` null "/KhaosIconMaker/Capture/M_InvertAlpha.M_InvertAlpha"))
  (set `self.ExportMaterial` _returnvalue)
  (`parent.UserConstructionScript`))