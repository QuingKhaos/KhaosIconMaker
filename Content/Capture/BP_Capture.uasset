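; Capture stage actor that spawns a single subject at the world origin: a buildable, an item's mesh or a raw static mesh.
; Each setter first destroys the previous subject through ClearCapture, then stores the new class and spawned actor.
; Buildables get LOD 0, huge cull distances, primary and secondary colors via custom primitive data, and a dynamic production indicator material tinted by state.
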(fn `ClearCapture`
  (bind _mbuildable (`self.mBuildable`))
  (bind _mstaticmesh (`self.mStaticMesh`))
  (`|ExecutionSequence`
    (:`then_0`
      (`/Engine/EditorBlueprintResources/StandardMacros.IsValid` _mbuildable
        (:`Is Valid`
          (`self.K2_DestroyActor` _mbuildable))))
    (:`then_1`
      (`/Engine/EditorBlueprintResources/StandardMacros.IsValid` _mstaticmesh
        (:`Is Valid`
          (`self.K2_DestroyActor` _mstaticmesh))))
    (:`then_2`
      (set `self.mClass` null))
    (:`then_3`
      (return))))

(fn `SetBuildableCapture`
  (params (Buildable :type "FGBuildable Class Reference") (PrimaryColor :type "LinearColor Structure") (SecondaryColor :type "LinearColor Structure") (ProductionIndicatorState :type "/KhaosIconMaker/EProductionIndicatorState Enum" :default "NewEnumerator1"))
  (bind (_primarycolor_r _primarycolor_g _primarycolor_b) (break `LinearColor` (`local.PrimaryColor`)))
  (bind (_secondarycolor_r _secondarycolor_g _secondarycolor_b) (break `LinearColor` (`local.SecondaryColor`)))
  (bind _array (`|MakeArray` _primarycolor_r _primarycolor_g _primarycolor_b _secondarycolor_r _secondarycolor_g _secondarycolor_b 0.0 0.0 0.0 0.0 0.0 0.0 0.0 0.0 0.0 0.0 0.0 0.0 0.0 0.0 0.0))
  (`self.ClearCapture`)
  (bind _output_get (set `self.mClass` Buildable))
  (bind _asactor (castclass `Actor` _output_get))
  (bind _returnvalue (`|SpawnActorFromClass` _asactor (`KismetMathLibrary.MakeTransform` (0.0 0.0 0.0)) "AlwaysSpawn" "MultiplyWithRoot" null null))
  (bind _asfgbuildable (cast `FGBuildable` _returnvalue))
  (bind _output_get_2 (set `self.mBuildable` _asfgbuildable))
  (`|ExecutionSequence`
    (:`then_0`
      (for _array_element (`self.K2_GetComponentsByClass` _output_get_2 "/Script/FactoryGame.FGColoredInstanceMeshProxy")
        (`StaticMeshComponent.SetForcedLodModel` _array_element 0)
        (`PrimitiveComponent.SetCullDistance` _array_element 5e+18)
        (`PrimitiveComponent.SetCustomPrimitiveDataFloatArray` _array_element 0 _array)))
    (:`then_1`
      (for _array_element_2 (`self.K2_GetComponentsByClass` _output_get_2 "/Script/Engine.SkeletalMeshComponent")
        (`SkinnedMeshComponent.SetForcedLOD` _array_element_2 0)
        (`PrimitiveComponent.SetCullDistance` _array_element_2 5e+18)
        (`PrimitiveComponent.SetCustomPrimitiveDataFloatArray` _array_element_2 0 _array)))
    (:`then_2`
      (for _array_element_3 (`self.K2_GetComponentsByClass` _output_get_2 "/Game/FactoryGame/Buildable/Factory/-Shared/ProductionIndicator/BP_ProductionIndicatorInstanced.BP_ProductionIndicatorInstanced_C")
        (bind _returnvalue_2 (`KismetMaterialLibrary.CreateDynamicMaterialInstance` "/KhaosIconMaker/Materials/MI_ProductionIndicator.MI_ProductionIndicator" (`KismetStringLibrary.Conv_StringToName` (`KismetStringLibrary.Concat_StrStr` "MI_ProductionIndicator_" (`KismetSystemLibrary.GetClassDisplayName` (`self.mClass`)))) "Transient"))
        (`MaterialInstanceDynamic.SetVectorParameterValue` _returnvalue_2 "EmissiveColor" (select `/KhaosIconMaker/EProductionIndicatorState` (`local.ProductionIndicatorState`) :`NewEnumerator1` (struct :`G` 1.0 :`A` 1.0) :`NewEnumerator2` (struct :`R` 0.14996 :`G` 0.254152 :`B` 0.752942 :`A` 1.0) :`NewEnumerator3` (struct :`R` 1.0 :`A` 1.0) :`NewEnumerator4` (struct :`R` 1.0 :`G` 1.0 :`A` 1.0) :!type "LinearColor Structure"))
        (`PrimitiveComponent.SetMaterial` _array_element_3 0 _returnvalue_2)))))

(fn `SetItemCapture`
  (params (ItemDesc :type "FGItemDescriptor Class Reference"))
  (`self.ClearCapture`)
  (set `self.mClass` ItemDesc)
  (bind _returnvalue (`|SpawnActorFromClass` "/Script/Engine.StaticMeshActor" (`KismetMathLibrary.MakeTransform` (0.0 0.0 0.0)) "AlwaysSpawn" "MultiplyWithRoot" null null))
  (`StaticMeshComponent.SetStaticMesh` (`StaticMeshActor.StaticMeshComponent` _returnvalue) (`FGItemDescriptor.GetItemMesh` ItemDesc))
  (set `self.mStaticMesh` _returnvalue)
  (return))

(fn `SetMeshCapture`
  (params (StaticMesh :type "StaticMesh Object Reference"))
  (`self.ClearCapture`)
  (set `self.mClass` (`GameplayStatics.GetObjectClass` StaticMesh))
  (bind _returnvalue (`|SpawnActorFromClass` "/Script/Engine.StaticMeshActor" (`KismetMathLibrary.MakeTransform` (0.0 0.0 0.0)) "AlwaysSpawn" "MultiplyWithRoot" null null))
  (`StaticMeshComponent.SetStaticMesh` (`StaticMeshActor.StaticMeshComponent` _returnvalue) StaticMesh)
  (set `self.mStaticMesh` _returnvalue)
  (return))

(fn `UserConstructionScript`)